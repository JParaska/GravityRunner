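; Game mode for an endless gravity runner that drives the Start, Play, Game Over and Revival states and their HUDs.
; Chains BP_Track segments from the last track's spawn point, scaling length with player max speed, and respawns them on a paid revive.
; Updates a save object with coins and run distances, which feed the game-over screen and last, best and average distance markers.
; Also handles coin-bought CameraLock and Magnet upgrades, saving those and revives to the slot.
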(event `self.ReceiveBeginPlay`
  (`parent.ReceiveBeginPlay`)
  (set `PlayerController.bShowMouseCursor` true (`GameplayStatics.GetPlayerController` 0))
  (`self.LoadGame`)
  (`GameplayStatics.PlaySound2D` null 1.0 1.0 0.0 null (`GameplayStatics.GetPlayerCharacter` 0))
  (`self.HandleGameState` "NewEnumerator0")
  (`self.SpawnDistanceMarkers`))

(event `self.ReceiveTick`
  (params (DeltaSeconds :type "Float (single-precision)"))
  (`parent.ReceiveTick` DeltaSeconds))

(fn `GameOverHUDValues`
  (params (GameOverHUD :type "/Game/HUD/GameOverHUD Object Reference"))
  (bind _highscorehud (`/Game/HUD/GameOverHUD.HighScoreHUD` GameOverHUD))
  (bind _savedgame (`self.SavedGame`))
  (bind _revivecost (`/Game/Blueprints/BP_SaveGame.ReviveCost` _savedgame))
  (`TextBlock.SetText` (`/Game/HUD/HighScoreHUD.LastRunValue` _highscorehud) (`KismetTextLibrary.Conv_DoubleToText` (`/Game/Blueprints/BP_SaveGame.LastDistance` _savedgame) "HalfToEven" false true 1 324 0 0))
  (`TextBlock.SetText` (`/Game/HUD/HighScoreHUD.LongestRunValue` _highscorehud) (`KismetTextLibrary.Conv_DoubleToText` (`/Game/Blueprints/BP_SaveGame.BestDistance` _savedgame) "HalfToEven" false true 1 324 0 0))
  (`TextBlock.SetText` (`/Game/HUD/HighScoreHUD.TotalCoinsValue` _highscorehud) (`KismetTextLibrary.Conv_IntToText` (`/Game/Blueprints/BP_SaveGame.Coins` _savedgame)))
  (`TextBlock.SetText` (`/Game/HUD/GameOverHUD.Revive` GameOverHUD) (`KismetTextLibrary.Conv_StringToText` (`KismetStringLibrary.Concat_StrStr` "Revive (" (`KismetStringLibrary.Conv_IntToString` _revivecost) ")")))
  (`Widget.SetIsEnabled` (`/Game/HUD/GameOverHUD.Button_Revive` GameOverHUD) (<= _revivecost (`/Game/Blueprints/BP_SaveGame.Coins` _savedgame)))
  (bind _asbp_gravity_runner_character (cast `/Game/Blueprints/BP_GravityRunnerCharacter` (`GameplayStatics.GetPlayerCharacter` 0)))
  (`TextBlock.SetText` (`/Game/HUD/HighScoreHUD.ColectedCoinsValue` _highscorehud) (`KismetTextLibrary.Conv_IntToText` (`/Game/Blueprints/BP_GravityRunnerCharacter.Coins` _asbp_gravity_runner_character))))

(fn `GameOverSetup`
  (params (State :type "/Game/Blueprints/E_GameState Enum" :default "NewEnumerator0"))
  (set `self.State` "NewEnumerator2")
  (`self.ManageSavedScore`)
  (`WidgetLayoutLibrary.RemoveAllWidgets`)
  (bind _returnvalue (`|CreateWidget` "/Game/HUD/GameOverHUD.GameOverHUD_C" (`GameplayStatics.GetPlayerController` 0)))
  (`UserWidget.AddToViewport` _returnvalue 0)
  (`GameplayStatics.SetGamePaused` true)
  (`self.GameOverHUDValues` _returnvalue))

(fn `GetCameraLockDuration`
  (returns (Duration :type "Float (double-precision)"))
  (bind _savedgame (`self.SavedGame`))
  (`/Engine/EditorBlueprintResources/StandardMacros.IsValid` _savedgame
    (:`Is Valid`
      (return (`.Duration_2_8B65A11F4D8A8F1AA1BF88B6F2E4F686` (break `/Game/Blueprints/FCameraLockData` (`/Game/Blueprints/BP_SaveGame.CameraLock` _savedgame)))))
    (:`Is Not Valid`
      (return 10.0))))

(fn `GetLockCameraNextLevelCost`
  (returns (Cost :type Integer))
  (bind _savedgame (`self.SavedGame`))
  (bind (_duration _level _maxlevel _levelcost) (break `/Game/Blueprints/FCameraLockData` (`/Game/Blueprints/BP_SaveGame.CameraLock` _savedgame)))
  (`/Engine/EditorBlueprintResources/StandardMacros.IsValid` _savedgame
    (:`Is Valid`
      (if (< _level _maxlevel)
        (return (`|GetArrayItem` _levelcost (+ _level 1)))))))

(fn `GetMagnetDuration`
  (returns (Duration :type "Float (double-precision)"))
  (bind _savedgame (`self.SavedGame`))
  (`/Engine/EditorBlueprintResources/StandardMacros.IsValid` _savedgame
    (:`Is Valid`
      (return (`.Duration_2_8B65A11F4D8A8F1AA1BF88B6F2E4F686` (break `/Game/Blueprints/FMagnetData` (`/Game/Blueprints/BP_SaveGame.Magnet` _savedgame)))))
    (:`Is Not Valid`
      (return 5.0))))

(fn `GetMagnetNextLevelCost`
  (returns (Cost :type Integer))
  (bind _savedgame (`self.SavedGame`))
  (bind (_duration _level _maxlevel _levelcost) (break `/Game/Blueprints/FMagnetData` (`/Game/Blueprints/BP_SaveGame.Magnet` _savedgame)))
  (`/Engine/EditorBlueprintResources/StandardMacros.IsValid` _savedgame
    (:`Is Valid`
      (if (< _level _maxlevel)
        (return (`|GetArrayItem` _levelcost (+ _level 1)))))))

(fn `GetTrackScale`
  (returns (ReturnValue :type "Float (double-precision)"))
  (bind _returnvalue (`MovementComponent.GetMaxSpeed` (`Character.CharacterMovement` (`GameplayStatics.GetPlayerCharacter` 0))))
  (if (<= _returnvalue 900.0)
    (return 1.0)
    (else
      (return (/ _returnvalue 900.0)))))

(fn `HandleGameState`
  (params (NewState :type "/Game/Blueprints/E_GameState Enum" :default "NewEnumerator0"))
  (switch `/Game/Blueprints/E_GameState` NewState
    (:`NewEnumerator0`
      (`self.MainMenuSetup`))
    (:`NewEnumerator1`
      (`self.StartGameSetup`))
    (:`NewEnumerator2`
      (`self.GameOverSetup` NewState))
    (:`NewEnumerator3`
      (`self.ReviveSetup`))))

(fn `IsCameraLockUpgradable`
  (returns (Upgradable :type Boolean))
  (bind _savedgame (`self.SavedGame`))
  (bind (_duration _level _maxlevel _levelcost) (break `/Game/Blueprints/FCameraLockData` (`/Game/Blueprints/BP_SaveGame.CameraLock` _savedgame)))
  (`/Engine/EditorBlueprintResources/StandardMacros.IsValid` _savedgame
    (:`Is Valid`
      (if (and (< _level _maxlevel) (not (>= _level (`KismetArrayLibrary.Array_Length` _levelcost))))
        (return (<= (`|GetArrayItem` _levelcost (+ _level 1)) (`/Game/Blueprints/BP_SaveGame.Coins` _savedgame)))
        (else
          (return false))))
    (:`Is Not Valid`
      (return false))))

(fn `IsMagnetUpgradable`
  (returns (Upgradable :type Boolean))
  (bind _savedgame (`self.SavedGame`))
  (bind (_duration _level _maxlevel _levelcost) (break `/Game/Blueprints/FMagnetData` (`/Game/Blueprints/BP_SaveGame.Magnet` _savedgame)))
  (`/Engine/EditorBlueprintResources/StandardMacros.IsValid` _savedgame
    (:`Is Valid`
      (if (and (< _level _maxlevel) (not (>= _level (`KismetArrayLibrary.Array_Length` _levelcost))))
        (return (<= (`|GetArrayItem` _levelcost (+ _level 1)) (`/Game/Blueprints/BP_SaveGame.Coins` _savedgame)))
        (else
          (return false))))
    (:`Is Not Valid`
      (return false))))

(fn `LoadGame`
  (bind _returnvalue (`GameplayStatics.LoadGameFromSlot` (`self.SaveGameSlotName`)))
  (`/Engine/EditorBlueprintResources/StandardMacros.IsValid` _returnvalue
    (:`Is Valid`
      (bind _asbp_save_game (cast `/Game/Blueprints/BP_SaveGame` _returnvalue))
      (set `self.SavedGame` _asbp_save_game))))

(fn `MainMenuSetup`
  (bind _returnvalue (`|CreateWidget` "/Game/HUD/MainMenuHUD.MainMenuHUD_C" (`GameplayStatics.GetPlayerController` 0)))
  (`UserWidget.AddToViewport` _returnvalue 0)
  (set `self.State` "NewEnumerator0"))

(fn `ManageSavedScore`
  (locals (TotalCoins :type Integer) (BestDistance :type "Float (double-precision)"))
  (bind _savedgame (`self.SavedGame`))
  (`/Engine/EditorBlueprintResources/StandardMacros.IsValid` _savedgame
    (:`Is Valid`
      (bind _output_get (set `local.TotalCoins` (`/Game/Blueprints/BP_SaveGame.Coins` _savedgame)))
      (bind _output_get_2 (set `local.BestDistance` (`/Game/Blueprints/BP_SaveGame.BestDistance` _savedgame))))
    (:`Is Not Valid`
      _))
  (`self.SaveGame` _output_get_2 _output_get))

(fn `ReviveSetup`
  (bind _returnvalue (`GameplayStatics.GetPlayerCharacter` 0))
  (bind _savedgame (`self.SavedGame`))
  (bind _savedgame_2 (`self.SavedGame`))
  ;[1 1 1] Handle revive cost
  (`/Engine/EditorBlueprintResources/StandardMacros.IsValid` _savedgame
    (:`Is Valid`
      (if (<= (`/Game/Blueprints/BP_SaveGame.ReviveCost` _savedgame) (`/Game/Blueprints/BP_SaveGame.Coins` _savedgame))
        (`/Game/Blueprints/BP_SaveGame.Revive` _savedgame_2)
        (`GameplayStatics.SaveGameToSlot` _savedgame_2 (`self.SaveGameSlotName`))
        (bind _asbp_gravity_runner_character (cast `/Game/Blueprints/BP_GravityRunnerCharacter` (`GameplayStatics.GetPlayerCharacter` 0)))
        (set `/Game/Blueprints/BP_GravityRunnerCharacter.Coins` 0 _asbp_gravity_runner_character)
        ;[1 1 1] Player location to center of tracks
        (`self.K2_SetActorLocation` _returnvalue (`KismetMathLibrary.MakeVector` (.x (`self.K2_GetActorLocation` _returnvalue))) false false)
        ;[1 1 1] HUD
        (`WidgetLayoutLibrary.RemoveAllWidgets`)
        (bind _returnvalue_2 (`|CreateWidget` "/Game/HUD/GameHUD.GameHUD_C" (`GameplayStatics.GetPlayerController` 0)))
        (`UserWidget.AddToViewport` _returnvalue_2 0)
        ;[1 1 1] Respawn tracks
        (bind _outactors (`GameplayStatics.GetAllActorsOfClass` "/Game/Blueprints/BP_Track.BP_Track_C"))
        (for _array_element _outactors
          (`self.K2_DestroyActor` _array_element))
        (bind _returnvalue_3 (`|SpawnActorFromClass` "/Game/Blueprints/BP_Track.BP_Track_C" (`KismetMathLibrary.MakeTransform` (`self.K2_GetActorLocation` (`GameplayStatics.GetPlayerCharacter` 0))) "AlwaysSpawn" "OverrideRootScale" null null))
        (set `self.LastTrack` _returnvalue_3)
        (`self.SpawnStartingracks` 6)
        ;[1 1 1] Unpause game
        (set `self.State` "NewEnumerator1")
        (`GameplayStatics.SetGamePaused` false)))))

(fn `SaveGame`
  (params (BestDistance :type "Float (double-precision)") (TotalCoins :type Integer))
  (bind _savedgame (`self.SavedGame`))
  (`/Engine/EditorBlueprintResources/StandardMacros.IsValid` (`self.SavedGame`)
    (:`Is Valid`
      _)
    (:`Is Not Valid`
      (bind _returnvalue (`GameplayStatics.CreateSaveGameObject` "/Game/Blueprints/BP_SaveGame.BP_SaveGame_C"))
      (set `self.SavedGame` _returnvalue)))
  (bind _asbp_gravity_runner_character (cast `/Game/Blueprints/BP_GravityRunnerCharacter` (`GameplayStatics.GetPlayerCharacter` 0)))
  (`self.SaveTotalCoins` TotalCoins _asbp_gravity_runner_character _savedgame)
  (`self.SaveLastDistance` _asbp_gravity_runner_character _savedgame)
  (`self.SaveLongestDistance` _asbp_gravity_runner_character BestDistance _savedgame)
  (set `self.SavedGame` _savedgame))

(fn `SaveLastDistance`
  (params (GRCharacter :type "/Game/Blueprints/BP_GravityRunnerCharacter Object Reference") (SaveGame :type "/Game/Blueprints/BP_SaveGame Object Reference"))
  (bind _output_get (set `/Game/Blueprints/BP_SaveGame.LastDistance` (`/Game/Blueprints/BP_GravityRunnerCharacter.RunDistance` GRCharacter) SaveGame))
  (`/Game/Blueprints/BP_SaveGame.AddDistance` SaveGame _output_get))

(fn `SaveLongestDistance`
  (params (GRCharacter :type "/Game/Blueprints/BP_GravityRunnerCharacter Object Reference") (LongestDistance :type "Float (double-precision)") (SaveGame :type "/Game/Blueprints/BP_SaveGame Object Reference"))
  (set `/Game/Blueprints/BP_SaveGame.BestDistance` (`KismetMathLibrary.FMax` (`/Game/Blueprints/BP_GravityRunnerCharacter.RunDistance` GRCharacter) LongestDistance) SaveGame))

(fn `SaveTotalCoins`
  (params (TotalCoins :type Integer) (GRCharacter :type "/Game/Blueprints/BP_GravityRunnerCharacter Object Reference") (SaveGame :type "/Game/Blueprints/BP_SaveGame Object Reference"))
  (set `/Game/Blueprints/BP_SaveGame.Coins` (+ TotalCoins (`/Game/Blueprints/BP_GravityRunnerCharacter.Coins` GRCharacter)) SaveGame))

(fn `SpawnDistanceMarker`
  (params (Distance :type "Float (double-precision)") (Label :type Text) (MarkerMaterial :type "MaterialInterface Object Reference"))
  (if (> Distance 0.0)
    (bind _returnvalue (`|SpawnActorFromClass` "/Game/Blueprints/BP_DistanceMarker.BP_DistanceMarker_C" (`KismetMathLibrary.MakeTransform` (`KismetMathLibrary.MakeVector` (* Distance 100.0))) "Undefined" "OverrideRootScale" null null))
    (`TextRenderComponent.K2_SetText` (`/Game/Blueprints/BP_DistanceMarker.DistanceLabel` _returnvalue) Label)
    (`TextRenderComponent.K2_SetText` (`/Game/Blueprints/BP_DistanceMarker.DistanceValue` _returnvalue) (`KismetTextLibrary.Conv_IntToText` (`KismetMathLibrary.FFloor` Distance)))
    (`/Game/Blueprints/BP_DistanceMarker.SetMarkerMaterial` _returnvalue MarkerMaterial)))

(fn `SpawnDistanceMarkers`
  (bind _savedgame (`self.SavedGame`))
  (`/Engine/EditorBlueprintResources/StandardMacros.IsValid` _savedgame
    (:`Is Valid`
      (`self.SpawnDistanceMarker` (`/Game/Blueprints/BP_SaveGame.LastDistance` _savedgame) "Last run" "/Engine/VREditor/BasicMeshes/MI_Cube_01.MI_Cube_01")
      (`self.SpawnDistanceMarker` (`/Game/Blueprints/BP_SaveGame.BestDistance` _savedgame) "Best run" "/Engine/VREditor/BasicMeshes/MI_Cube_02.MI_Cube_02")
      (`self.SpawnDistanceMarker` (`/Game/Blueprints/BP_SaveGame.GetAverageDistance` _savedgame) "Average run" "/Engine/VREditor/BasicMeshes/MI_Cube_03.MI_Cube_03"))))

(fn `SpawnStartingracks`
  (params (Number :type Integer :default 3))
  (for _ (range (+ Number 1))
    (`self.SpawnTrack` 6)))

(fn `SpawnTrack`
  (params (MinPlatforms :type Integer :default 6) (MaxPlatforms :type Integer :default 6))
  (locals (SpawnLocation :type "Vector Structure"))
  (bind _lasttrack (`self.LastTrack`))
  (`/Engine/EditorBlueprintResources/StandardMacros.IsValid` _lasttrack
    (:`Is Valid`
      (bind _output_get (set `local.SpawnLocation` (`SceneComponent.K2_GetComponentLocation` (`/Game/Blueprints/BP_Track.SpawnPoint` _lasttrack)))))
    (:`Is Not Valid`
      _))
  (bind _returnvalue (`|SpawnActorFromClass` "/Game/Blueprints/BP_Track.BP_Track_C" (`KismetMathLibrary.MakeTransform` _output_get (struct :`Yaw` 180.0) (`KismetMathLibrary.MakeVector` (`self.GetTrackScale`) 1.0 1.0)) "Undefined" "OverrideRootScale" null null))
  (`/Game/Blueprints/BP_Track.CreatePlatforms` _returnvalue MinPlatforms MaxPlatforms)
  (bind _output_get_2 (set `self.LastTrack` _returnvalue))
  (`PrimitiveComponent.SetCollisionEnabled` (`/Game/Blueprints/BP_Track.DestroyTrigger` _output_get_2) "QueryOnly")
  (`PrimitiveComponent.SetCollisionEnabled` (`/Game/Blueprints/BP_Track.SpawnTrigger` _output_get_2) "QueryOnly"))

(fn `StartGameSetup`
  (if (`|EnumEquality` (`self.State`) "NewEnumerator2")
    (`GameplayStatics.OpenLevel` "Game"))
  (`WidgetLayoutLibrary.RemoveAllWidgets`)
  (`self.SpawnStartingracks` 3)
  (bind _returnvalue (`|CreateWidget` "/Game/HUD/GameHUD.GameHUD_C" (`GameplayStatics.GetPlayerController` 0)))
  (`UserWidget.AddToViewport` _returnvalue 0)
  (set `self.State` "NewEnumerator1"))

(fn `UpgradeCameraLock`
  (bind _savedgame (`self.SavedGame`))
  (bind _savedgame_2 (`self.SavedGame`))
  (bind (_duration _level _maxlevel _levelcost) (break `/Game/Blueprints/FCameraLockData` (`/Game/Blueprints/BP_SaveGame.CameraLock` _savedgame)))
  (`/Engine/EditorBlueprintResources/StandardMacros.IsValid` _savedgame
    (:`Is Valid`
      (if (< _level _maxlevel)
        (bind _result (`/Engine/EditorBlueprintResources/StandardMacros.IncrementInt` _level)
          (:`  `
            (bind _result_2 (`/Engine/EditorBlueprintResources/StandardMacros.DecrementFloat` _duration)
              (:`  `
                (set `/Game/Blueprints/BP_SaveGame.CameraLock` (make `/Game/Blueprints/FCameraLockData` _result_2 _result 5 _levelcost) _savedgame_2)
                (set `/Game/Blueprints/BP_SaveGame.Coins` (- (`/Game/Blueprints/BP_SaveGame.Coins` _savedgame_2) (`|GetArrayItem` _levelcost _result)) (`self.SavedGame`))
                (`GameplayStatics.SaveGameToSlot` (`self.SavedGame`) (`self.SaveGameSlotName`))))))))))

(fn `UpgradeMagnet`
  (bind _savedgame (`self.SavedGame`))
  (bind _savedgame_2 (`self.SavedGame`))
  (bind (_duration _level _maxlevel _levelcost) (break `/Game/Blueprints/FMagnetData` (`/Game/Blueprints/BP_SaveGame.Magnet` _savedgame)))
  (`/Engine/EditorBlueprintResources/StandardMacros.IsValid` _savedgame
    (:`Is Valid`
      (if (< _level _maxlevel)
        (bind _result (`/Engine/EditorBlueprintResources/StandardMacros.IncrementInt` _level)
          (:`  `
            (bind _result_2 (`/Engine/EditorBlueprintResources/StandardMacros.IncrementFloat` _duration)
              (:`  `
                (set `/Game/Blueprints/BP_SaveGame.Magnet` (make `/Game/Blueprints/FMagnetData` _result_2 _result 5 _levelcost) _savedgame_2)
                (set `/Game/Blueprints/BP_SaveGame.Coins` (- (`/Game/Blueprints/BP_SaveGame.Coins` _savedgame_2) (`|GetArrayItem` _levelcost _result)) (`self.SavedGame`))
                (`GameplayStatics.SaveGameToSlot` (`self.SavedGame`) (`self.SaveGameSlotName`))))))))))

(fn `UserConstructionScript`
  (`parent.UserConstructionScript`))