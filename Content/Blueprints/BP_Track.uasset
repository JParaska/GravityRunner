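; BP_Track is a track segment for the gravity runner that randomly fills up to six upper and lower platform slots.
; CreatePlatforms sets meshes on a unique random selection of slots, then rolls coin or rare camera-lock pickups at each platform's three sockets.
; Player overlaps drive the flow: SpawnTrigger asks the game mode for more track, DestroyTrigger destroys this segment, and six boxes report a game-state change.
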(event `self.DestroyTrigger.OnComponentBeginOverlap`
  (params (OverlappedComponent :type "PrimitiveComponent Object Reference") (OtherActor :type "Actor Object Reference") (OtherComp :type "PrimitiveComponent Object Reference") (OtherBodyIndex :type Integer) (bFromSweep :type Boolean) (SweepResult :type "HitResult Structure (by ref)"))
  (if (== OtherActor (`GameplayStatics.GetPlayerCharacter` 0))
    (`self.K2_DestroyActor`)))

(event `self.SpawnTrigger.OnComponentBeginOverlap`
  (params (OverlappedComponent :type "PrimitiveComponent Object Reference") (OtherActor :type "Actor Object Reference") (OtherComp :type "PrimitiveComponent Object Reference") (OtherBodyIndex :type Integer) (bFromSweep :type Boolean) (SweepResult :type "HitResult Structure (by ref)"))
  (if (== OtherActor (`GameplayStatics.GetPlayerCharacter` 0))
    (bind _asbp_gravity_runner_gm (cast `/Game/Blueprints/BP_GravityRunnerGM` (`GameplayStatics.GetGameMode`)))
    (`/Game/Blueprints/BP_GravityRunnerGM.SpawnTrack` _asbp_gravity_runner_gm 3 5)))

(event `self.Box.OnComponentBeginOverlap`
  (params (OverlappedComponent :type "PrimitiveComponent Object Reference") (OtherActor :type "Actor Object Reference") (OtherComp :type "PrimitiveComponent Object Reference") (OtherBodyIndex :type Integer) (bFromSweep :type Boolean) (SweepResult :type "HitResult Structure (by ref)"))
  (if (== OtherActor (`GameplayStatics.GetPlayerCharacter` 0))
    (bind _asbp_gravity_runner_gm (cast `/Game/Blueprints/BP_GravityRunnerGM` (`GameplayStatics.GetGameMode`) :!label _label))
    (`/Game/Blueprints/BP_GravityRunnerGM.HandleGameState` _asbp_gravity_runner_gm "NewEnumerator2")))

(event `self.Box1.OnComponentBeginOverlap`
  (params (OverlappedComponent :type "PrimitiveComponent Object Reference") (OtherActor :type "Actor Object Reference") (OtherComp :type "PrimitiveComponent Object Reference") (OtherBodyIndex :type Integer) (bFromSweep :type Boolean) (SweepResult :type "HitResult Structure (by ref)"))
  (if (== OtherActor (`GameplayStatics.GetPlayerCharacter` 0))
    (goto _label)))

(event `self.Box2.OnComponentBeginOverlap`
  (params (OverlappedComponent :type "PrimitiveComponent Object Reference") (OtherActor :type "Actor Object Reference") (OtherComp :type "PrimitiveComponent Object Reference") (OtherBodyIndex :type Integer) (bFromSweep :type Boolean) (SweepResult :type "HitResult Structure (by ref)"))
  (if (== OtherActor (`GameplayStatics.GetPlayerCharacter` 0))
    (goto _label)))

(event `self.Box3.OnComponentBeginOverlap`
  (params (OverlappedComponent :type "PrimitiveComponent Object Reference") (OtherActor :type "Actor Object Reference") (OtherComp :type "PrimitiveComponent Object Reference") (OtherBodyIndex :type Integer) (bFromSweep :type Boolean) (SweepResult :type "HitResult Structure (by ref)"))
  (if (== OtherActor (`GameplayStatics.GetPlayerCharacter` 0))
    (goto _label)))

(event `self.Box4.OnComponentBeginOverlap`
  (params (OverlappedComponent :type "PrimitiveComponent Object Reference") (OtherActor :type "Actor Object Reference") (OtherComp :type "PrimitiveComponent Object Reference") (OtherBodyIndex :type Integer) (bFromSweep :type Boolean) (SweepResult :type "HitResult Structure (by ref)"))
  (if (== OtherActor (`GameplayStatics.GetPlayerCharacter` 0))
    (goto _label)))

(event `self.Box5.OnComponentBeginOverlap`
  (params (OverlappedComponent :type "PrimitiveComponent Object Reference") (OtherActor :type "Actor Object Reference") (OtherComp :type "PrimitiveComponent Object Reference") (OtherBodyIndex :type Integer) (bFromSweep :type Boolean) (SweepResult :type "HitResult Structure (by ref)"))
  (if (== OtherActor (`GameplayStatics.GetPlayerCharacter` 0))
    (goto _label)))

(fn `ChoosePickup`
  (returns (NewParam :type "/Game/Blueprints/Pickups/BP_Pickup Class Reference"))
  (if (<= (`KismetMathLibrary.RandomFloat`) 0.02)
    (return "/Game/Blueprints/Pickups/BP_Pickup_CameraLock.BP_Pickup_CameraLock_C")
    (else
      (return "/Game/Blueprints/Pickups/BP_Pickup_Coin.BP_Pickup_Coin_C"))))

(fn `CreatePlatforms`
  (params (Min :type Integer :default 6) (Max :type Integer :default 6))
  (locals (SpawnedPlatform :type Integer))
  (bind _downcenter (`self.DownCenter`))
  (bind _upleft (`self.UpLeft`))
  (bind _downright (`self.DownRight`))
  (bind _downleft (`self.DownLeft`))
  (bind _upcenter (`self.UpCenter`))
  (bind _upright (`self.UpRight`))
  (bind _pick (`self.PickPlatforms` (`KismetMathLibrary.RandomIntegerInRange` Min Max)))
  (for _array_element _pick
    (switch `int` _array_element
      (:`Default`
        (`StaticMeshComponent.SetStaticMesh` _upleft (`self.Mesh`) :!label _label)
        (`self.SpawnPickup` _upleft))
      (:`0`
        (`StaticMeshComponent.SetStaticMesh` _downcenter (`self.Mesh`))
        (`self.SpawnPickup` _downcenter))
      (:`1`
        (`StaticMeshComponent.SetStaticMesh` _downright (`self.Mesh`))
        (`self.SpawnPickup` _downright))
      (:`2`
        (`StaticMeshComponent.SetStaticMesh` _downleft (`self.Mesh`))
        (`self.SpawnPickup` _downleft))
      (:`3`
        (`StaticMeshComponent.SetStaticMesh` _upcenter (`self.Mesh`))
        (`self.SpawnPickup` _upcenter))
      (:`4`
        (`StaticMeshComponent.SetStaticMesh` _upright (`self.Mesh`))
        (`self.SpawnPickup` _upright))
      (:`5`
        (goto _label)))))

(fn `PickPlatforms`
  (params (Number :type Integer))
  (returns (Pick :type "Array of Integer"))
  (locals (PickedPlatforms :type "Array of Integer"))
  (while true :!label _label
    (`KismetArrayLibrary.Array_AddUnique` (`local.PickedPlatforms`) (`KismetMathLibrary.RandomIntegerInRange` 0 5))
    (if true
      (if (== (`KismetArrayLibrary.Array_Length` (`local.PickedPlatforms`)) Number)
        (return (`local.PickedPlatforms`))
        (else
          (goto _label))))))

(fn `RandomPickupSpawn`
  (params (Platform :type "SceneComponent Object Reference") (SocketName :type Name))
  (if (>= (`KismetMathLibrary.RandomFloat`) 0.5)
    (bind _newparam (`self.ChoosePickup`))
    (`|SpawnActorFromClass` _newparam (`KismetMathLibrary.MakeTransform` (`SceneComponent.GetSocketLocation` Platform SocketName) (`SceneComponent.GetSocketRotation` Platform SocketName)) "Undefined" "OverrideRootScale" null null)))

(fn `SpawnPickup`
  (params (Platform :type "StaticMeshComponent Object Reference"))
  (`self.RandomPickupSpawn` Platform "PickupSocket01")
  (`self.RandomPickupSpawn` Platform "PickupSocket02")
  (`self.RandomPickupSpawn` Platform "PickupSocket03"))

(fn `UserConstructionScript`
  (`parent.UserConstructionScript`))