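; BP_SaveGame is a save-game Blueprint that tracks run distances, coins and the cost of reviving.
; AddDistance appends to AllDistances, which GetAverageDistance is meant to average.
; Its length check is inverted: it averages only an empty array and returns -1 whenever distances exist.
; Revive deducts ReviveCost from Coins without a balance check, then raises the cost by 20 percent, rounded down.
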(fn `AddDistance`
  (params (Distance :type "Float (double-precision)"))
  (`KismetArrayLibrary.Array_Add` (`self.AllDistances`) Distance))

(fn `GetAverageDistance`
  (returns (AverageDistance :type "Float (double-precision)"))
  (locals (TotalDistance :type "Float (double-precision)"))
  (if (== (`KismetArrayLibrary.Array_Length` (`self.AllDistances`)) 0)
    (for _array_element (`self.AllDistances`)
      (set `local.TotalDistance` (+ _array_element (`local.TotalDistance`))))
    (return (/ (`local.TotalDistance`) (`KismetMathLibrary.Conv_IntToDouble` (`KismetArrayLibrary.Array_Length` (`self.AllDistances`)))))
    (else
      (return -1.0))))

(fn `Revive`
  (set `self.Coins` (- (`self.Coins`) (`self.ReviveCost`)))
  (set `self.ReviveCost` (`KismetMathLibrary.FFloor` (* (`self.ReviveCost`) 1.2))))