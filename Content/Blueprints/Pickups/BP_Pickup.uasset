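; BP_Pickup is a base pickup actor for the gravity runner, collected when the player character overlaps its Collision component.
; On BeginPlay it casts its owner to BP_Track and binds to that track's BeforeDestroy, so it is destroyed along with the track.
; On overlap it calls CollectPickup with the player and destroys itself; child Blueprints override that function, which here only prints a reminder.
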(event `self.ReceiveBeginPlay`
  (bind _asbp_track (cast `/Game/Blueprints/BP_Track` (`self.GetOwner`)))
  (add `/Game/Blueprints/BP_Track.BeforeDestroy` _asbp_track (delegate `OnDestroy`)))

(event `OnDestroy`
  (`self.K2_DestroyActor`))

(event `self.Collision.OnComponentBeginOverlap`
  (params (OverlappedComponent :type "PrimitiveComponent Object Reference") (OtherActor :type "Actor Object Reference") (OtherComp :type "PrimitiveComponent Object Reference") (OtherBodyIndex :type Integer) (bFromSweep :type Boolean) (SweepResult :type "HitResult Structure (by ref)"))
  (if (== OtherActor (`GameplayStatics.GetPlayerCharacter` 0))
    (bind _asbp_gravity_runner_character (cast `/Game/Blueprints/BP_GravityRunnerCharacter` OtherActor))
    (`self.CollectPickup` _asbp_gravity_runner_character)
    (`self.K2_DestroyActor`)))

(fn `CollectPickup`
  (params (Player :type "/Game/Blueprints/BP_GravityRunnerCharacter Object Reference"))
  (`KismetSystemLibrary.PrintString` "Override in child BP"))

(fn `UserConstructionScript`)