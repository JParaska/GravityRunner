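; BP_Pickup_Coin is a coin pickup that credits the collecting player.
; Its CollectPickup event calls CollectCoin on the passed-in player, then spawns a half-scale pixel explosion particle effect, reusing an enemy explosion template, at the coin's location.
; BeginPlay, overlap and Tick are disabled stubs, and the construction script only calls its parent, so this graph holds no detection or removal logic.
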(event `self.CollectPickup`
  (params (Player :type "/Game/Blueprints/BP_GravityRunnerCharacter Object Reference"))
  (`/Game/Blueprints/BP_GravityRunnerCharacter.CollectCoin` Player)
  (`GameplayStatics.SpawnEmitterAtLocation` "/Game/Assets/Effects/P_Pixel_Explosion_Enemy.P_Pixel_Explosion_Enemy" (.location (`self.GetTransform`)) (.rotation (`self.GetTransform`)) (0.5 0.5 0.5)))

(fn `UserConstructionScript`
  (`parent.UserConstructionScript`))