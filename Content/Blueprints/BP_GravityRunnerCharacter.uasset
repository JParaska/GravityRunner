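; Player character for a gravity runner that auto-runs forward during the Play state, gaining speed while tracking distance and coins.
; Left/Right input, usable only when grounded and not switching, jumps and selects the linked neighboring track point.
; Tick interpolates Y/Z toward that point while blending the GravityMovementComponent's gravity to its forward vector.
; The camera eases between start, play and game-over anchors according to BP_GravityRunnerGM's state.
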(event `Key|A`
  (params (Key :type "Key Structure"))
  ;[1 1 1] TESTInput
  (:`Pressed`
    (`self.Left` :!label _label)))

(event `Key|Left`
  (params (Key :type "Key Structure"))
  ;[1 1 1] TESTInput
  (:`Pressed`
    (goto _label)))

(event `Key|D`
  (params (Key :type "Key Structure"))
  ;[1 1 1] TESTInput
  (:`Pressed`
    (`self.Right` :!label _label_2)))

(event `Key|Right`
  (params (Key :type "Key Structure"))
  ;[1 1 1] TESTInput
  (:`Pressed`
    (goto _label_2)))

(event `Right`
  (bind _right (`/Game/Blueprints/BP_TrackPoint.Right` (`self.ActualTrackPoint`)))
  ;[0.2761 1 0.4838] Input
  (if (`self.IsNotMoving`)
    (`self.Jump`)
    (set `self.End` (`self.K2_GetActorLocation` _right))
    (set `self.ActualTrackPoint` _right)
    (set `self.Moving` true :!label _label_3)))

(event `Left`
  (bind _left (`/Game/Blueprints/BP_TrackPoint.Left` (`self.ActualTrackPoint`)))
  ;[0.2761 1 0.4838] Input
  (if (`self.IsNotMoving`)
    (`self.Jump`)
    (set `self.End` (`self.K2_GetActorLocation` _left))
    (set `self.ActualTrackPoint` _left)
    (goto _label_3)))

(event `Key|SpaceBar`
  (params (Key :type "Key Structure"))
  ;[0.2761 1 0.4838] Input
)

(event `self.ReceiveTick`
  (params (DeltaSeconds :type "Float (single-precision)"))
  (`parent.ReceiveTick` DeltaSeconds)
  (`|ExecutionSequence`
    (:`then_0`
      (bind _asbp_gravity_runner_gm (cast `/Game/Blueprints/BP_GravityRunnerGM` (`GameplayStatics.GetGameMode`)))
      (if (`|EnumEquality` (`/Game/Blueprints/BP_GravityRunnerGM.State` _asbp_gravity_runner_gm) "NewEnumerator1")
        (`self.AddMovementInput` (`self.GetActorForwardVector`))))
    (:`then_1`
      (if (`self.Moving`)
        (`self.ChangeTrack` DeltaSeconds)))
    (:`then_2`
      (`self.IncreaseSpeed` DeltaSeconds))
    (:`then_3`
      (`self.MeasureRunDistance` DeltaSeconds))
    (:`then_4`
      (`self.PlayerCamera` DeltaSeconds))))

(fn `ChangeTrack`
  (params (DeltaTime :type "Float (double-precision)"))
  (bind (_x _y) (`KismetMathLibrary.BreakVector2D` (`KismetMathLibrary.Vector2DInterpTo` (`KismetMathLibrary.MakeVector2D` (.y (`self.K2_GetActorLocation`)) (.z (`self.K2_GetActorLocation`))) (`KismetMathLibrary.MakeVector2D` (.y (`self.End`)) (.z (`self.End`))) DeltaTime 5.0)))
  (`self.K2_SetActorLocation` (`KismetMathLibrary.MakeVector` (.x (`self.K2_GetActorLocation`)) _x _y) false true)
  (bind _asgravity_movement_component (cast `GravityMovementComponent` (`self.CharacterMovement`)))
  (`GravityMovementComponent.SetGravityDirection` _asgravity_movement_component (`KismetMathLibrary.VInterpTo` (`GravityMovementComponent.GetGravityDirection` _asgravity_movement_component false) (`self.GetActorForwardVector` (`self.ActualTrackPoint`)) DeltaTime 10.0))
  (if (== (`KismetMathLibrary.MakeVector2D` (.y (`self.K2_GetActorLocation`)) (.z (`self.K2_GetActorLocation`))) (`KismetMathLibrary.MakeVector2D` (.y (`self.End`)) (.z (`self.End`))) :`ErrorTolerance` 5.0)
    (`self.K2_SetActorLocation` (`KismetMathLibrary.MakeVector` (.x (`self.K2_GetActorLocation`)) (`.Y` (`KismetMathLibrary.BreakVector2D` (`KismetMathLibrary.Conv_VectorToVector2D` (`self.End`)))) (.z (`self.K2_GetActorLocation`))) false true)
    (`GravityMovementComponent.SetGravityDirection` _asgravity_movement_component (`self.GetActorForwardVector` (`self.ActualTrackPoint`)))
    (set `self.Moving` false)))

(fn `CollectCoin`
  (`/Engine/EditorBlueprintResources/StandardMacros.IncrementInt` (`self.Coins`)))

(fn `IncreaseSpeed`
  (params (DeltaSpeed :type "Float (double-precision)"))
  (bind _charactermovement (`self.CharacterMovement`))
  (set `CharacterMovementComponent.MaxWalkSpeed` (+ (* DeltaSpeed 10.0) (`CharacterMovementComponent.MaxWalkSpeed` _charactermovement)) _charactermovement))

(fn `IsNotMoving`
  (returns (ReturnValue :type Boolean))
  (return (not (or (`self.Moving`) (`NavMovementComponent.IsFalling` (`self.CharacterMovement`))))))

(fn `LockCameraRoll`
  (`SceneComponent.K2_SetRelativeRotation` :`self` (`self.SpringArm`))
  (set `SpringArmComponent.bInheritRoll` true (`self.SpringArm`)))

(fn `MeasureRunDistance`
  (params (DeltaSeconds :type "Float (double-precision)"))
  (set `self.RunDistance` (+ (* DeltaSeconds (/ (`MovementComponent.GetMaxSpeed` (`self.CharacterMovement`)) 100.0)) (`self.RunDistance`) 0.0)))

(fn `PlayerCamera`
  (params (DeltaTime :type "Float (double-precision)"))
  (bind _asbp_gravity_runner_gm (cast `/Game/Blueprints/BP_GravityRunnerGM` (`GameplayStatics.GetGameMode`)))
  (bind _returnvalue (select `/Game/Blueprints/E_GameState` (`/Game/Blueprints/BP_GravityRunnerGM.State` _asbp_gravity_runner_gm) :`NewEnumerator0` (`self.GCPoint`) :`NewEnumerator1` (`self.MCPoint`) :`NewEnumerator2` (`self.GOCPoint`)))
  (`SceneComponent.K2_SetWorldLocation` (`self.Camera`) (`KismetMathLibrary.VInterpTo` (`SceneComponent.K2_GetComponentLocation` (`self.Camera`)) (`SceneComponent.K2_GetComponentLocation` _returnvalue) DeltaTime 1.0) false false)
  (`SceneComponent.K2_SetWorldRotation` (`self.Camera`) (`KismetMathLibrary.RInterpTo` (`SceneComponent.K2_GetComponentRotation` (`self.Camera`)) (`SceneComponent.K2_GetComponentRotation` _returnvalue) DeltaTime 3.0) false false))

(fn `UnlockCamerRoll`
  (`SceneComponent.K2_SetRelativeRotation` (`self.SpringArm`) (`SceneComponent.K2_GetComponentRotation` (`self.CapsuleComponent`)) false false)
  (set `SpringArmComponent.bInheritRoll` false (`self.SpringArm`)))

(fn `UserConstructionScript`
  (`parent.UserConstructionScript`))